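; BP_EnemyCharacter is an enemy NPC character that takes damage and can die.
; On any damage it plays a hit reaction montage and subtracts the damage from Health, inside an IsGettingHit guard that clears immediately without waiting for the montage.
; When Health reaches zero or below, it disables capsule collision, sets IsDead and clamps Health to zero.
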(event `self.ReceiveTick`
  (params (DeltaSeconds :type "Float (single-precision)")))

(event `self.ReceiveAnyDamage`
  (params (Damage :type "Float (single-precision)") (DamageType :type "DamageType Object Reference") (InstigatedBy :type "Controller Object Reference") (DamageCauser :type "Actor Object Reference"))
  ;[1 1 1] What to do if we recivce Damage
  (if (not (`self.bIsGettingHit`))
    (set `self.bIsGettingHit` true)
    (`self.PlayAnimMontage` "/Game/Animations/NPC/EnemyCharacter/Reactions/HitReactionMontage.HitReactionMontage")
    (bind _output_get (set `self.Health` (- (`self.Health`) Damage)))
    (set `self.bIsGettingHit` false)
    (if (<= _output_get 0.0)
      (`PrimitiveComponent.SetCollisionEnabled` (`self.CapsuleComponent`) "NoCollision")
      (set `self.bIsDead` true)
      (set `self.Health` 0.0))))

(fn `UserConstructionScript`)